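; BP_COLL_ADN is a DNA (ADN) collectible that the ThirdPersonCharacter picks up by walking into its box collision.
; Each pickup spawns a scene actor, calls Iniciar with the No_ADN entry matching the pickup's order, then destroys itself.
; It then increments the character's ContadorAdn, and the fourth pickup sets ObjetivoADN and prints an objective-complete message.
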(event OnComponentBeginOverlap(BoxCollision)
  (params (OverlappedComponent :type Primitive%20Component%20Object%20Reference) (OtherActor :type Actor%20Object%20Reference) (OtherComp :type Primitive%20Component%20Object%20Reference) (OtherBodyIndex :type Integer) (bFromSweep :type Boolean) (SweepResult :type Hit%20Result%20Structure%20%28by%20ref%29))
  (bind _asthird_person_character (Utilities|Casting|CastToThirdPersonCharacter OtherActor))
  (if (== (+ (Variables|/Game/BP/ThirdPersonCharacter.ThirdPersonCharacter_C|GetContador_adn _asthird_person_character) 1) 1)
    (bind _returnvalue (Game|SpawnActorfromClass "/Game/BP/PlantillaEscena.PlantillaEscena_C" (Math|Transform|MakeTransform "0, 0, 0" "0, 0, 0" "1,1,1") "Undefined" 0 0))
    (bind _output_get (Variables|Default|SetEscena%20Actual _returnvalue))
    (Default|Iniciar _output_get "/Game/Dialogos/No_ADN_1.No_ADN_1")
    (Actor|DestroyActor self)
    (Variables|/Game/BP/ThirdPersonCharacter.ThirdPersonCharacter_C|SetContador_adn _asthird_person_character (+ (Variables|/Game/BP/ThirdPersonCharacter.ThirdPersonCharacter_C|GetContador_adn _asthird_person_character) 1) :!label _label)
    (if (== (Variables|/Game/BP/ThirdPersonCharacter.ThirdPersonCharacter_C|GetContador_adn _asthird_person_character) 4)
      (Variables|/Game/BP/ThirdPersonCharacter.ThirdPersonCharacter_C|SetObjetivo_ADN _asthird_person_character true)
      (Development|PrintString "Objetivo Completo"))
    (elif (== (+ (Variables|/Game/BP/ThirdPersonCharacter.ThirdPersonCharacter_C|GetContador_adn _asthird_person_character) 1) 2)
      (bind _returnvalue_2 (Game|SpawnActorfromClass "/Game/BP/PlantillaEscena.PlantillaEscena_C" (Math|Transform|MakeTransform "0, 0, 0" "0, 0, 0" "1,1,1") "Undefined" 0 0))
      (bind _output_get_2 (Variables|Default|SetEscena%20Actual _returnvalue_2))
      (Default|Iniciar _output_get_2 "/Game/Dialogos/No_ADN_2.No_ADN_2")
      (Actor|DestroyActor self)
      (goto _label)
      (elif (== (+ (Variables|/Game/BP/ThirdPersonCharacter.ThirdPersonCharacter_C|GetContador_adn _asthird_person_character) 1) 3)
        (bind _returnvalue_3 (Game|SpawnActorfromClass "/Game/BP/PlantillaEscena.PlantillaEscena_C" (Math|Transform|MakeTransform "0, 0, 0" "0, 0, 0" "1,1,1") "Undefined" 0 0))
        (bind _output_get_3 (Variables|Default|SetEscena%20Actual _returnvalue_3))
        (Default|Iniciar _output_get_3 "/Game/Dialogos/No_ADN_3.No_ADN_3")
        (Actor|DestroyActor self)
        (goto _label)
        (elif (== (+ (Variables|/Game/BP/ThirdPersonCharacter.ThirdPersonCharacter_C|GetContador_adn _asthird_person_character) 1) 4)
          (bind _returnvalue_4 (Game|SpawnActorfromClass "/Game/BP/PlantillaEscena.PlantillaEscena_C" (Math|Transform|MakeTransform "0, 0, 0" "0, 0, 0" "1,1,1") "Undefined" 0 0))
          (bind _output_get_4 (Variables|Default|SetEscena%20Actual _returnvalue_4))
          (Default|Iniciar _output_get_4 "/Game/Dialogos/No_ADN_4.No_ADN_4")
          (Actor|DestroyActor self)
          (goto _label))))))

(event EventBeginPlay)

(event Collision|EventActorBeginOverlap
  (params (OtherActor :type Actor%20Object%20Reference))
  (Utilities|Casting|CastToThirdPersonCharacter OtherActor))

(event EventTick
  (params (DeltaSeconds :type Float%20%28single-precision%29)))

(fn ConstructionScript)